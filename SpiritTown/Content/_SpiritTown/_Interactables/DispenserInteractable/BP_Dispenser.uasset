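; BP_Dispenser is an interactable that dispenses a new actor each time it is interacted with.
; It extends its parent's InteractingEvent to call DispenseNewObject, which spawns the ActorToDispense class just above the dispenser's root, regardless of collisions.
; It then immediately sends an Interact interface message to the spawned actor, so the new object is interacted with as soon as it appears.
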(event EventBeginPlay
  (|CallParentFunction) ; This node is disabled and will not be called.\nDrag off pins to build functionality.
)

(event Collision|EventActorBeginOverlap
  (params (OtherActor :type Actor%20Object%20Reference))
  (|CallParentFunction OtherActor) ; This node is disabled and will not be called.\nDrag off pins to build functionality.
)

(event EventTick
  (params (DeltaSeconds :type Float%20%28single-precision%29))
  (|CallParentFunction DeltaSeconds) ; This node is disabled and will not be called.\nDrag off pins to build functionality.
)

(event EventInteractingEvent
  (|CallParentFunction)
  (CallFunction|DispenseNewObject))

(fn ConstructionScript
  (|CallParentFunction))

(fn DispenseNewObject
  (bind _defaultsceneroot (Variables|Default|GetDefaultSceneRoot))
  (bind _returnvalue (Transformation|GetWorldLocation _defaultsceneroot))
  (bind _returnvalue_2 (Game|SpawnActorfromClass (Variables|Dispenser|GetActorToDispense) (Math|Conversions|ToTransform(Vector) (Math|Vector|MakeVector (.x _returnvalue) (.y _returnvalue) (+ (.z _returnvalue) 1e+02))) "AlwaysSpawn" 0 0))
  (Class|IInteractables|IInteract(Message) _returnvalue_2))