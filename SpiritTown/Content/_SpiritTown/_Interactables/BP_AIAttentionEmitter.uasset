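; Attention emitter that draws BP_BaseNPC characters' attention to its owning actor for a set time.
; EmitDistraction notifies the listed specific actors, then, unless restricted to that list, NPCs found by a debug-drawn sphere trace around the owner.
; The one-time guard checks EmmitedOnce, but that flag is set only on the repeatable branch, so one-time emission never sets it.
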(event EventBeginPlay)

(event EventTick
  (params (DeltaSeconds :type Float%20%28single-precision%29)))

(fn EmitGeneralDistraction
  (bind _owningactor (Variables|Default|GetOwningActor))
  (bind _rootcomponent (Variables|/Script/Engine.Actor|GetRootComponent _owningactor))
  (bind _returnvalue (Transformation|GetWorldLocation _rootcomponent))
  (bind (_x _y _z) (Math|Vector|BreakVector _returnvalue))
  (bind (_outhits _returnvalue_2) (Collision|MultiSphereTraceByChannel (Math|Vector|MakeVector _x _y _z) (Math|Vector|MakeVector _x _y (+ _z 1e+01)) (Variables|Default|GetAttentionCaptureRadius) "TraceTypeQuery5" false 0 "ForDuration"))
  (if _returnvalue_2
    (bind _output_get (LocalVariables|SetHits _outhits))
    (bind _array_element (Utilities|Array|ForEachLoopwithBreak _output_get)
      (:LoopBody
        (Utilities|IsValid (.hitactor _array_element)
          (:Is%20Valid
            (bind _asbp_base_npc (Utilities|Casting|CastToBP_BaseNPC (.hitactor _array_element)))
            (Default|AttentionBeingGrabbed _asbp_base_npc (Variables|Default|GetOwningActor) (Variables|Default|GetAttentionCaptureTime))))))))

(fn EmitSpecificActors
  (if (Utilities|Array|IsValidIndex (Variables|Default|GetSpecifcActors))
    (for _array_element (Variables|Default|GetSpecifcActors)
      (bind _asbp_base_npc (Utilities|Casting|CastToBP_BaseNPC _array_element))
      (Default|AttentionBeingGrabbed _asbp_base_npc (Variables|Default|GetOwningActor) (Variables|Default|GetAttentionCaptureTime)))))

(fn EmitDistraction
  (if (Variables|Default|GetOneTimeEmitter)
    (if (not (Variables|Default|GetEmmitedOnce))
      (CallFunction|EmitSpecificActors :!label _label)
      (if (not (Variables|Default|GetOnly%20Use%20Specific%20Actors))
        (CallFunction|EmitGeneralDistraction)))
    (else
      (Variables|Default|SetEmmitedOnce true)
      (goto _label))))