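; BP_carryInteracble is a carryable-interaction target in Spirit Town that fills toward completion when interacted with by an actor whose class is in KeyItem.
; Each accepted interaction adds FillRate to CurrentCapacity and updates the progress widget assigned through SetObjectUIREF.
; It completes when one more increment would reach RequiredCapacity, then notifies its MasterObject and the widget.
; Getters expose the widget class, reference, placement and activation state.
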(event Custom|OnInteract
  (if (> (Variables|Default|GetRequired%20Capacity) 0.0)
    (CallFunction|AddtoCapcity)))

(event Custom|RequirementMet
  (Variables|Default|SetComplete true)
  (Utilities|IsValid (Variables|Default|GetMasterObject)
    (:Is%20Valid
      (Class|IMasterObject|ChildComplete(Message) (Variables|Default|GetMasterObject) self))))

(event EventBeginPlay)

(event Collision|EventActorBeginOverlap
  (params (OtherActor :type Actor%20Object%20Reference)))

(event EventTick
  (params (DeltaSeconds :type Float%20%28single-precision%29)))

(event EventICarryableInteraction
  (params (Interactor :type Actor%20Object%20Reference))
  (if (not (Variables|Default|GetComplete))
    (if (Utilities|Array|ContainsItem (Variables|Default|GetKeyItem) (Utilities|GetClass Interactor))
      (CallFunction|OnInteract))))

(event EventSetObjectUIREF
  (params (CreateUI :type User%20Widget%20Object%20Reference))
  (Variables|Default|SetInteractWidgetREF CreateUI))

(fn ConstructionScript)

(fn AddtoCapcity
  (Variables|Default|SetCurrentCapacity (+ (Variables|Default|GetCurrentCapacity) (Variables|Default|GetFillRate)))
  (CallFunction|SetWorldSpaceProgress)
  (if (>= (+ (Variables|Default|GetCurrentCapacity) (Variables|Default|GetFillRate)) (Variables|Default|GetRequired%20Capacity))
    (Variables|Default|SetCurrentCapacity (Variables|Default|GetRequired%20Capacity))
    (CallFunction|RequirementMet)
    (Class|IWorldSpaceUI|CompleteEvent(Message) (Variables|Default|GetInteractWidgetREF))))

(fn SetWorldSpaceProgress
  (bind _required_capacity (Variables|Default|GetRequired%20Capacity))
  (bind _currentcapacity (Variables|Default|GetCurrentCapacity))
  (bind _returnvalue (/ _currentcapacity _required_capacity))
  (Utilities|IsValid (Variables|Default|GetInteractWidgetREF)
    (:Is%20Valid
      (LocalVariables|SetFillProgress 0.0)
      (if (> _returnvalue 1.0)
        (LocalVariables|SetFillProgress 1.0)
        (else
          (LocalVariables|SetFillProgress _returnvalue)))
      (Class|IWorldSpaceUI|SetHoldingProgress(Message) (Variables|Default|GetInteractWidgetREF) (LocalVariables|GetFillProgress)))))

(fn GetifHasActivated
  (return (Variables|Default|GetActivatedState)))

(fn GetObjectUICLASS
  (return (Variables|Default|GetInteractWidgetClass)))

(fn GetObjectUIREF
  (return (Variables|Default|GetInteractWidgetREF)))

(fn GetWorldSpacePlacement
  (return (Variables|Default|GetInteractWidgetPlacement)))