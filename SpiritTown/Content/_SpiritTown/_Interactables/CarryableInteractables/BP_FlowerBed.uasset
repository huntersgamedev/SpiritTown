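; BP_FlowerBed is an interactable flower bed that tracks completion of its child flower patches.
; On BeginPlay it sets itself as MasterObject on each patch key in the FlowerPatches map.
; ChildComplete marks a patch done, shows a completed/total count on the interact widget, then fires its completion message and sets "Water" text when all are done.
; Getters supply the widget's class, reference and world-space placement.
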(event EventBeginPlay
  (bind _keys (Utilities|Map|Keys (Variables|Default|GetFlowerPatches)))
  (for _array_element _keys
    (Variables|/Game/_SpiritTown/_Interactables/CarryableInteractables/BP_carryInteracble.BP_carryInteracble_C|SetMasterObject _array_element self)))

(event Collision|EventActorBeginOverlap
  (params (OtherActor :type Actor%20Object%20Reference)))

(event EventTick
  (params (DeltaSeconds :type Float%20%28single-precision%29)))

(event EventChildComplete
  (params (ChildCompleted :type Actor%20Object%20Reference))
  (bind _interactwidgetref (Variables|Default|GetInteractWidgetRef))
  (Utilities|Map|Add (Variables|Default|GetFlowerPatches) (.AsBP%20Flower%20Patch (Utilities|Casting|CastToBP_FlowerPatch ChildCompleted)) true)
  (bind _allcompleted (CallFunction|SetAmountCompleted))
  (if _allcompleted
    (Class|IWorldSpaceUI|CompleteEvent(Message) _interactwidgetref)
    (Class|IWorldSpaceUI|SetTextItem1(Message) _interactwidgetref "Water")))

(event EventSetObjectUIREF
  (params (CreateUI :type User%20Widget%20Object%20Reference))
  (Variables|Default|SetInteractWidgetRef CreateUI))

(fn ConstructionScript)

(fn CheckifBedComplete
  (LocalVariables|SetNotCompete false)
  (bind _keys (Utilities|Map|Keys (Variables|Default|GetFlowerPatches)))
  (bind _array_element (Utilities|Array|ForEachLoopwithBreak _keys :!label _label)
    (:LoopBody
      (if (not (.Value (Utilities|Map|Find (Variables|Default|GetFlowerPatches) _array_element)))
        (LocalVariables|SetNotCompete true)
        (goto _label Break)))
    (:Completed
      (return (not (LocalVariables|GetNotCompete))))))

(fn SetAmountCompleted
  (LocalVariables|SetAmountCompleted 0)
  (bind _keys (Utilities|Map|Keys (Variables|Default|GetFlowerPatches)))
  (bind _array_element (Utilities|Array|ForEachLoopwithBreak _keys)
    (:LoopBody
      (if (.Value (Utilities|Map|Find (Variables|Default|GetFlowerPatches) _array_element))
        (Math|Integer|IncrementInt (LocalVariables|GetAmountCompleted))))
    (:Completed
      (Utilities|IsValid (Variables|Default|GetInteractWidgetRef)
        (:Is%20Valid
          (if (>= (LocalVariables|GetAmountCompleted) (Utilities|Map|Length (Variables|Default|GetFlowerPatches)))
            _
            (else
              (Class|IWorldSpaceUI|SetTextItem1(Message) (Variables|Default|GetInteractWidgetRef) (Utilities|Text|ToText(String) (Utilities|String|Append (Utilities|String|ToString(Integer) (LocalVariables|GetAmountCompleted)) "/" (Utilities|String|ToString(Integer) (Utilities|Map|Length (Variables|Default|GetFlowerPatches)))))))))
        (:Is%20Not%20Valid
          _))
      (return (>= (LocalVariables|GetAmountCompleted) (Utilities|Map|Length (Variables|Default|GetFlowerPatches)))))))

(fn GetifHasActivated
  (return false))

(fn GetObjectUICLASS
  (return (Variables|Default|GetInteractWidgetClass)))

(fn GetObjectUIREF
  (return (Variables|Default|GetInteractWidgetRef)))

(fn GetWorldSpacePlacement
  (return (Variables|Default|GetInteractWidgetPlacement)))