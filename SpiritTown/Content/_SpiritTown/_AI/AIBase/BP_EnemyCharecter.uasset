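; Enemy character base that patrols waypoints and chases the player, with spawner-tracked NPC types that can despawn near an end location.
; PawnSensing starts a chase after a range check, ignoring breath-holding players unless it can detect them.
; Tick drops the chase when facing, distance or line-trace checks fail.
; Chase state drives the AI Blackboard and walk/run speed, while patrol helpers supply the next point and wait time.
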(event OnSeePawn(PawnSensing)
  (params (Pawn :type Pawn%20Object%20Reference))
  (if (Utilities|InRange?Idle Pawn)
    (if (Variables|Default|GetCanDetectBreathHeld)
      (CallFunction|SetChase true :!label _label)
      (elif (not (Variables|/Game/_SpiritTown/_Player/PlayerBP_LittleOneV2.PlayerBP_LittleOneV2_C|GetHolding%20Breath (.AsPlayer%20BP%20Little%20One%20V2 (Utilities|Casting|CastToPlayerBP_LittleOneV2 Pawn))))
        (goto _label)))))

(event EventBeginPlay)

(event Collision|EventActorBeginOverlap
  (params (OtherActor :type Actor%20Object%20Reference)))

(event EventTick
  (params (DeltaSeconds :type Float%20%28single-precision%29))
  (CallFunction|DebugSightDistance)
  (CallFunction|CheckIFSeesPlayer))

(fn ConstructionScript)

(fn GiveNextPatrolLocation
  (Math|Integer|IncrementInt (Variables|Default|GetPoint%20In%20Patrol)
    (:%20%20
      (if (> (Variables|Default|GetPoint%20In%20Patrol) (- (Utilities|Array|Length (Variables|Default|GetPatrol%20Locations)) 1))
        (Variables|Default|SetPoint%20In%20Patrol 0)
        (CallFunction|Despawn))
      (bind _asbp_patrol_locations (Utilities|Casting|CastToBP_PatrolLocations (Utilities|Array|Get(acopy) (Variables|Default|GetPatrol%20Locations) (Variables|Default|GetPoint%20In%20Patrol)))
        (:then
          (LocalVariables|SetSetWaitTime (Variables|/Game/_SpiritTown/_AI/AIBase/BP_PatrolLocations.BP_PatrolLocations_C|GetWaittime _asbp_patrol_locations)))
        (:CastFailed
          (LocalVariables|SetSetWaitTime 0.5)))
      (return (LocalVariables|GetSetWaitTime) _asbp_patrol_locations))))

(fn DebugSightDistance
  (if (Variables|Default|GetDebugShow%20SightDistance)
    (Utilities|FlowControl|Sequence
      (:then_0
        (Development|PrintString (Utilities|String|Append "Detection Distance  is:" (Utilities|String|ToString(Float) (Variables|Default|GetSightDistance))))
        (Development|PrintString (Utilities|String|Append "Player distance is:" (Utilities|String|ToString(Float) (Transformation|GetDistanceTo (Game|GetPlayerCharacter 0))))))
      (:then_1
        (Rendering|Debug|DrawDebugSphere (+ (Transformation|GetWorldLocation (Variables|Collision|GetCapsuleComponent)) (* (Math|Vector|GetForwardVector "0, 0, 0") (Variables|Default|GetSightDistance))) 3e+01 12 "(R=1.000000,G=0.782358,B=0.000000,A=1.000000)" 1.0 1.0)))))

(fn SetmovementSpeed
  (params (Speed :type ENU_Speed%20Enum :default "NewEnumerator0"))
  (switch Utilities|FlowControl|Switch|SwitchonENU_Speed Speed
    (:NewEnumerator0
      (Variables|/Script/Engine.CharacterMovementComponent|SetMaxWalkSpeed (Variables|Character|GetCharacterMovement) (Variables|Locomotion|GetDoddleSpeed)))
    (:NewEnumerator1
      (Variables|/Script/Engine.CharacterMovementComponent|SetMaxWalkSpeed (Variables|Character|GetCharacterMovement) (Variables|Locomotion|GetWalkSpeed)))
    (:NewEnumerator2
      (Variables|/Script/Engine.CharacterMovementComponent|SetMaxWalkSpeed (Variables|Character|GetCharacterMovement) (Variables|Locomotion|GetRunSpeed)))))

(fn CheckIFSeesPlayer
  (if (Math|Boolean|ANDBoolean (.isFacingEachother (Utilities|ISFacingObject (Transformation|GetWorldLocation (Variables|/Script/Engine.Character|GetCapsuleComponent (Game|GetPlayerCharacter 0))) (Transformation|GetWorldLocation (Variables|Collision|GetCapsuleComponent)) (Math|Vector|GetForwardVector (Variables|Collision|GetCapsuleComponent)) 0.0)) (< (Transformation|GetDistanceTo (Game|GetPlayerCharacter 0)) (Variables|Default|GetAlertSightDistance)) (Variables|Default|GetdoesSeePlayer))
    (bind _outhit (Collision|LineTraceByChannel (Transformation|GetWorldLocation (Variables|Default|GetFaceMarker)) (Transformation|GetWorldLocation (Variables|/Script/Engine.Character|GetCapsuleComponent (Game|GetPlayerCharacter 0))) "TraceTypeQuery2" false 0 "ForDuration"))
    (bind _output_get (LocalVariables|SetTrace1Actor (.hitactor _outhit)))
    (Utilities|IsValid _output_get
      (:Is%20Valid
        (if (!= (LocalVariables|GetTrace1Actor) (Game|GetPlayerCharacter 0))
          (CallFunction|SetChase false)))
      (:Is%20Not%20Valid
        (CallFunction|SetChase false)))
    (else
      (CallFunction|SetChase false))))

(fn SetChase
  (params (IsSeeingPlayer :type Boolean))
  (Variables|Default|SetdoesSeePlayer IsSeeingPlayer)
  (AI|Components|Blackboard|SetValueasBool (Variables|/Script/AIModule.AIController|GetBlackboard (AI|GetAIController self)) (Variables|Default|Getseesplayer) IsSeeingPlayer)
  (if IsSeeingPlayer
    (CallFunction|SetmovementSpeed "NewEnumerator2")
    (else
      (CallFunction|SetmovementSpeed "NewEnumerator1"))))

(fn Despawn
  (if (and (Variables|Default|GetDespawn?) (< (Transformation|GetDistanceTo (Variables|Default|GetEndLocation)) 2.5e+02))
    (switch Utilities|FlowControl|Switch|SwitchonENU_CrowdType (Variables|Default|Get%20NPC%20Type)
      (:NewEnumerator0
        (Math|Integer|DecrementInt (Variables|/Game/_SpiritTown/_AI/AIBase/Spawners/NPCSpawner.NPCSpawner_C|GetCurrent%20Stream%20Amount (Variables|Default|GetSpawner))
          (:%20%20
            _)))
      (:NewEnumerator1
        (Math|Integer|DecrementInt (Variables|/Game/_SpiritTown/_AI/AIBase/Spawners/NPCSpawner.NPCSpawner_C|GetCurrent%20StoreGoerAmount (Variables|Default|GetSpawner))
          (:%20%20
            _))))
    (Actor|DestroyActor))
  (return))