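; Base NPC character that patrols, spots and chases the player, and searches after losing them, with behavior varied by a trait list.
; Pawn sensing and periodic forward sphere traces start chases, factoring in player stealth.
; Per-tick soft or hard pursuit checks facing, range and line of sight, writing chase state to the Blackboard.
; Helpers supply patrol points, build nearest-first search routes from nearby nodes, and despawn spawner-counted NPCs at route end.
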(event OnSeePawn(PawnSensing)
  (params (Pawn :type Pawn%20Object%20Reference))
  (bind _asplayer_bp_little_one_v2 (Utilities|Casting|CastToPlayerBP_LittleOneV2 Pawn))
  (if (CallFunction|CheckforTrait "NewEnumerator5")
    (if (Utilities|InRange?Idle Pawn)
      (if (Variables|/Game/_SpiritTown/_Player/PlayerBP_LittleOneV2.PlayerBP_LittleOneV2_C|GetHiding _asplayer_bp_little_one_v2)
        (CallFunction|SetChase true :!label _label)
        (elif (not (Variables|/Game/_SpiritTown/_Player/PlayerBP_LittleOneV2.PlayerBP_LittleOneV2_C|GetHolding%20Breath _asplayer_bp_little_one_v2))
          (goto _label))))))

(event EventBeginPlay
  (if (CallFunction|CheckforTrait "NewEnumerator5")
    (Components|DestroyComponent (Variables|Default|GetDecal)))
  (Utilities|IsValid (Utilities|Array|Get(acopy) (Variables|Default|GetPatrol%20Locations))
    (:Is%20Not%20Valid
      (bind _returnvalue (Game|SpawnActorfromClass "/Game/_SpiritTown/_AI/AIBase/BP_PatrolLocations.BP_PatrolLocations_C" (Math|Conversions|ToTransform(Vector) (Transformation|GetWorldLocation (Variables|Character|GetMesh))) "Undefined" 0 0))
      (Utilities|Array|Add (Variables|Default|GetPatrol%20Locations) _returnvalue))))

(event Collision|EventActorBeginOverlap
  (params (OtherActor :type Actor%20Object%20Reference)))

(event EventTick
  (params (DeltaSeconds :type Float%20%28single-precision%29))
  (Variables|Default|SetDelataTime DeltaSeconds)
  (CallFunction|FormSight)
  (if (CallFunction|CheckforTrait "NewEnumerator0")
    (CallFunction|SoftPursuitSight)
    (else
      (CallFunction|HardPursuitSight))))

(fn ConstructionScript
  (if (Variables|Debug|GetShowFormSight)
    (Variables|Debug|SetShowFormSight false)
    (CallFunction|DebugDrawFormSight)))

(fn GiveNextPatrolLocation
  (Math|Integer|IncrementInt (Variables|Default|GetPoint%20In%20Patrol)
    (:%20%20
      (if (> (Variables|Default|GetPoint%20In%20Patrol) (- (Utilities|Array|Length (Variables|Default|GetPatrol%20Locations)) 1))
        (Variables|Default|SetPoint%20In%20Patrol 0)
        (CallFunction|Despawn))
      (bind _asbp_patrol_locations (Utilities|Casting|CastToBP_PatrolLocations (Utilities|Array|Get(acopy) (Variables|Default|GetPatrol%20Locations) (Variables|Default|GetPoint%20In%20Patrol)))
        (:then
          (LocalVariables|SetSetWaitTime (Variables|/Game/_SpiritTown/_AI/AIBase/BP_PatrolLocations.BP_PatrolLocations_C|GetWaittime _asbp_patrol_locations)))
        (:CastFailed
          (LocalVariables|SetSetWaitTime 0.5)))
      (return (LocalVariables|GetSetWaitTime) _asbp_patrol_locations))))

(fn DebugSightDistance
  (if (Variables|Default|GetDebugShow%20SightDistance)
    (Utilities|FlowControl|Sequence
      (:then_0
        (Development|PrintString (Utilities|String|Append "Detection Distance  is:" (Utilities|String|ToString(Float) (Variables|Default|GetSightDistance))))
        (Development|PrintString (Utilities|String|Append "Player distance is:" (Utilities|String|ToString(Float) (Transformation|GetDistanceTo (Game|GetPlayerCharacter 0))))))
      (:then_1
        (Rendering|Debug|DrawDebugSphere (+ (Transformation|GetWorldLocation (Variables|Collision|GetCapsuleComponent)) (* (Math|Vector|GetForwardVector "0, 0, 0") (Variables|Default|GetSightDistance))) 3e+01 12 "(R=1.000000,G=0.782358,B=0.000000,A=1.000000)" 1.0 1.0)))))

(fn SetmovementSpeed
  (params (Speed :type ENU_Speed%20Enum :default "NewEnumerator0"))
  (Variables|/Script/Engine.CharacterMovementComponent|SetMaxWalkSpeed (Variables|Character|GetCharacterMovement) (.Value (Utilities|Map|Find (Variables|Default|GetNpcMovementSpeeds) Speed))))

(fn SoftPursuitSight
  (if (Variables|Default|GetdoesSeePlayer)
    (if (and (.isFacingEachother (Utilities|ISFacingObject (Transformation|GetWorldLocation (Variables|/Script/Engine.Character|GetCapsuleComponent (Game|GetPlayerCharacter 0))) (Transformation|GetWorldLocation (Variables|Collision|GetCapsuleComponent)) (Math|Vector|GetForwardVector (Variables|Collision|GetCapsuleComponent)) 0.0)) (< (Transformation|GetDistanceTo (Game|GetPlayerCharacter 0)) (Variables|Default|GetSOFTAlertSightDistance)))
      (bind _outhit (Collision|LineTraceByChannel (Transformation|GetWorldLocation (Variables|Default|GetFaceMarker)) (Transformation|GetWorldLocation (Variables|/Script/Engine.Character|GetCapsuleComponent (Game|GetPlayerCharacter 0))) "TraceTypeQuery2" false 0 "None"))
      (bind _output_get (LocalVariables|SetTrace1Actor (.hitactor _outhit)))
      (Utilities|IsValid _output_get
        (:Is%20Valid
          (if (!= (LocalVariables|GetTrace1Actor) (Game|GetPlayerCharacter 0))
            (CallFunction|SetChase false)))
        (:Is%20Not%20Valid
          (CallFunction|SetChase false)))
      (else
        (CallFunction|SetChase false)))))

(fn SetChase
  (params (IsSeeingPlayer :type Boolean))
  (Variables|Default|SetdoesSeePlayer IsSeeingPlayer)
  (AI|Components|Blackboard|SetValueasBool (Variables|/Script/AIModule.AIController|GetBlackboard (AI|GetAIController self)) (Variables|Default|Getseesplayer) IsSeeingPlayer)
  (if IsSeeingPlayer
    (CallFunction|ChangeStatus "NewEnumerator1")
    (CallFunction|SetmovementSpeed "NewEnumerator2")
    (elif (CallFunction|CheckforTrait "NewEnumerator0")
      (CallFunction|ChangeStatus "NewEnumerator0" :!label _label)
      (CallFunction|SetmovementSpeed "NewEnumerator1")
      (elif (Variables|Default|GetIgnoreHardPursuit)
        (Variables|Default|SetIgnoreHardPursuit false)
        (goto _label)
        (else
          (CallFunction|SetLastSighted)
          (CallFunction|ChangeStatus "NewEnumerator2"))))))

(fn Despawn
  (if (and (Variables|Default|GetDespawn?) (< (Transformation|GetDistanceTo (Variables|Default|GetEndLocation)) 2.5e+02))
    (switch Utilities|FlowControl|Switch|SwitchonENU_CrowdType (Variables|traits|GetNPC%20Type)
      (:NewEnumerator0
        (Math|Integer|DecrementInt (Variables|/Game/_SpiritTown/_AI/AIBase/Spawners/NPCSpawner.NPCSpawner_C|GetCurrent%20Stream%20Amount (Variables|Default|GetSpawner))
          (:%20%20
            _)))
      (:NewEnumerator1
        (Math|Integer|DecrementInt (Variables|/Game/_SpiritTown/_AI/AIBase/Spawners/NPCSpawner.NPCSpawner_C|GetCurrent%20StoreGoerAmount (Variables|Default|GetSpawner))
          (:%20%20
            _))))
    (Actor|DestroyActor))
  (return))

(fn CheckforTrait
  (params (TraitToSearch :type NPC_Traits%20Enum :default "NewEnumerator0"))
  (LocalVariables|SetTraitSearchingFor TraitToSearch)
  (LocalVariables|SetFoundTrait false)
  (bind _array_element (Utilities|Array|ForEachLoopwithBreak (Variables|traits|GetTRAITS) :!label _label)
    (:LoopBody
      (if (== _array_element (LocalVariables|GetTraitSearchingFor))
        (LocalVariables|SetFoundTrait true)
        (goto _label Break)))
    (:Completed
      (return (LocalVariables|GetFoundTrait)))))

(fn FormSight
  (bind _mesh (Variables|Character|GetMesh))
  (bind _capsulecomponent (Variables|Collision|GetCapsuleComponent))
  (bind _formsightoffset (Variables|FormSight|GetFormSightOffset))
  (bind _returnvalue (Math|Vector|GetForwardVector _capsulecomponent))
  (bind _returnvalue_2 (Transformation|GetWorldLocation _mesh))
  (bind _returnvalue_3 (* _returnvalue _formsightoffset))
  (bind _returnvalue_4 (+ _returnvalue_2 _returnvalue_3))
  (bind _output_get (Variables|FormSight|SetCurrentFormSightTime (+ (Variables|FormSight|GetCurrentFormSightTime) (Variables|Default|GetDelataTime))))
  (if (>= _output_get (Variables|FormSight|GetFormSightCheckRate))
    (Variables|FormSight|SetCurrentFormSightTime 0.0)
    (if (CallFunction|CheckforTrait "NewEnumerator4")
      (if (Variables|Default|GetDebugShow%20SightDistance)
        (Rendering|Debug|DrawDebugSphere (+ (Transformation|GetWorldLocation (Variables|Character|GetMesh)) (* (Math|Vector|GetForwardVector (Variables|Collision|GetCapsuleComponent)) (Variables|FormSight|GetFormSightOffset))) (Variables|FormSight|GetFormSightRadius) 12 "(R=0.992503,G=0.000000,B=1.000000,A=1.000000)" 0.2 0.5))
      (bind _outhits (Collision|MultiSphereTraceByChannel (Math|Vector|MakeVector (.x _returnvalue_4) (.y _returnvalue_4) (.z _returnvalue_4)) (Math|Vector|MakeVector (.x _returnvalue_4) (.y _returnvalue_4) (+ (.z _returnvalue_4) (Variables|FormSight|GetFormSensingHeight))) (Variables|FormSight|GetFormSightRadius) "TraceTypeQuery3" true 0 "None"))
      (bind _array_element (Utilities|Array|ForEachLoopwithBreak _outhits :!label _label)
        (:LoopBody
          (LocalVariables|SetSeenActor (.hitactor _array_element))
          (if (== (.hitactor _array_element) (Game|GetPlayerCharacter 0))
            (if (not (Variables|/Game/_SpiritTown/_Player/PlayerBP_LittleOneV2.PlayerBP_LittleOneV2_C|GetHiding (.AsPlayer%20BP%20Little%20One%20V2 (Utilities|Casting|CastToPlayerBP_LittleOneV2 (LocalVariables|GetSeenActor)))))
              (CallFunction|SetChase true)
              (goto _label Break))))))))

(fn DebugDrawFormSight
  (Rendering|Debug|DrawDebugSphere (+ (Transformation|GetWorldLocation (Variables|Character|GetMesh)) (* (Math|Vector|GetForwardVector (Variables|Collision|GetCapsuleComponent)) (Variables|FormSight|GetFormSightOffset))) (Variables|FormSight|GetFormSightRadius) 12 "(R=0.992503,G=0.000000,B=1.000000,A=1.000000)" 3e+01 0.5))

(fn SightConfirm
  (bind _outhit (Collision|LineTraceByChannel (Transformation|GetWorldLocation (Variables|Default|GetFaceMarker)) (Transformation|GetWorldLocation (Variables|/Script/Engine.Character|GetCapsuleComponent (Game|GetPlayerCharacter 0))) "TraceTypeQuery2" false 0 "None"))
  (bind _output_get (LocalVariables|SetTraceActor (.hitactor _outhit)))
  (bind _asplayer_bp_little_one_v2 (Utilities|Casting|CastToPlayerBP_LittleOneV2 _output_get))
  (if (not (Variables|/Game/_SpiritTown/_Player/PlayerBP_LittleOneV2.PlayerBP_LittleOneV2_C|GetHiding _asplayer_bp_little_one_v2))
    (CallFunction|SetChase true)))

(fn HardPursuitSight
  (if (Variables|Default|GetdoesSeePlayer)
    (if (and (.isFacingEachother (Utilities|ISFacingObject (Transformation|GetWorldLocation (Variables|/Script/Engine.Character|GetCapsuleComponent (Game|GetPlayerCharacter 0))) (Transformation|GetWorldLocation (Variables|Collision|GetCapsuleComponent)) (Math|Vector|GetForwardVector (Variables|Collision|GetCapsuleComponent)) 0.0)) (< (Transformation|GetDistanceTo (Game|GetPlayerCharacter 0)) (Variables|Default|GetHARDAlertSightDistance)))
      (bind _outhit (Collision|LineTraceByChannel (Transformation|GetWorldLocation (Variables|Default|GetFaceMarker)) (Transformation|GetWorldLocation (Variables|/Script/Engine.Character|GetCapsuleComponent (Game|GetPlayerCharacter 0))) "TraceTypeQuery2" false 0 "None"))
      (bind _output_get (LocalVariables|SetTrace1Actor (.hitactor _outhit)))
      (Utilities|IsValid _output_get
        (:Is%20Valid
          (if (!= (LocalVariables|GetTrace1Actor) (Game|GetPlayerCharacter 0))
            (CallFunction|SetChase false)))
        (:Is%20Not%20Valid
          (CallFunction|SetChase false)))
      (else
        (CallFunction|SetChase false)))))

(fn ChangeStatus
  (params (new%20status :type NPCStatus%20Enum :default "NewEnumerator0"))
  (bind _output_get (Variables|traits|SetCurrentStatus new%20status))
  (AI|Components|Blackboard|SetValueasEnum (Variables|/Script/AIModule.AIController|GetBlackboard (AI|GetAIController self)) (Variables|Default|GetStatus) _output_get))

(fn SetLastSighted
  (Variables|Default|SetLastSightedLocation (Transformation|GetWorldLocation (Variables|/Script/Engine.Character|GetMesh (Game|GetPlayerCharacter 0)))))

(fn TraceforSearchLocations
  (bind _mesh (Variables|Character|GetMesh))
  (bind _returnvalue (Transformation|GetWorldLocation _mesh))
  (bind (_x _y _z) (Math|Vector|BreakVector _returnvalue))
  (bind _outhits (Collision|MultiSphereTraceByChannel (Math|Vector|MakeVector _x _y _z) (Math|Vector|MakeVector _x _y (+ _z (Variables|FormSight|GetFormSensingHeight))) (Variables|Default|GetSearchRadius) "TraceTypeQuery3" true 0 "ForDuration"))
  (Utilities|IsValid (.hitactor (Utilities|Array|Get(acopy) _outhits))
    (:Is%20Valid
      (Variables|Default|SetSEarchpoints true)
      (for _array_element _outhits
        (bind _asbp_patrol_locations (Utilities|Casting|CastToBP_PatrolLocations (.hitactor _array_element)))
        (Variables|Default|SetTracedSearchNode _asbp_patrol_locations)
        (if (Utilities|Enum|Equal(Enum) (Variables|/Game/_SpiritTown/_AI/AIBase/BP_PatrolLocations.BP_PatrolLocations_C|GetNodeType (Variables|Default|GetTracedSearchNode)) "NewEnumerator1")
          (Utilities|Array|Add (Variables|Default|GetSearchNodesNearby) (Variables|Default|GetTracedSearchNode))))
      (Utilities|IsValid (Utilities|Array|Get(acopy) (Variables|Default|GetSearchNodesNearby))
        (:Is%20Valid
          (CallFunction|CreateSearchRoute))
        (:Is%20Not%20Valid
          (Variables|Default|SetSEarchpoints false :!label _label))))
    (:Is%20Not%20Valid
      (goto _label)))
  (return (Variables|Default|GetSEarchpoints)))

(fn CreateSearchRoute
  (for _index (range 0 (Math|Random|RandomIntegerinRange 1 (- (Utilities|Array|Length (Variables|Default|GetSearchNodesNearby)) 1)))
    (for (_array_element _array_index) (Variables|Default|GetSearchNodesNearby)
      (Variables|Default|SetCurrentSearchNode _array_element)
      (if (== _array_index 0)
        (Variables|Default|SetOptimalDistance (Math|Vector|Distance(Vector) (Transformation|GetActorLocation self) (Transformation|GetActorLocation (Variables|Default|GetCurrentSearchNode))))
        (Variables|Default|SetSearchNodeNodeToAdd (Variables|Default|GetCurrentSearchNode))
        (elif (not (< (Variables|Default|GetOptimalDistance) (Math|Vector|Distance(Vector) (Transformation|GetActorLocation self) (Transformation|GetActorLocation (Variables|Default|GetCurrentSearchNode)))))
          (Variables|Default|SetSearchNodeNodeToAdd (Variables|Default|GetCurrentSearchNode))
          (Variables|Default|SetOptimalDistance (Math|Vector|Distance(Vector) (Transformation|GetActorLocation self) (Transformation|GetActorLocation (Variables|Default|GetCurrentSearchNode)))))))
    (Utilities|Array|Add (Variables|Default|GetSearchRoute) (Variables|Default|GetSearchNodeNodeToAdd))
    (Utilities|Array|RemoveItem (Variables|Default|GetSearchNodesNearby) (Variables|Default|GetSearchNodeNodeToAdd))))

(fn GiveNextSearchLocation
  (Math|Integer|IncrementInt (Variables|Default|GetPointInSearch)
    (:%20%20
      (LocalVariables|SetLastLocation false)
      (if (> (Variables|Default|GetPointInSearch) (- (Utilities|Array|Length (Variables|Default|GetSearchRoute)) 1))
        (LocalVariables|SetLastLocation true))
      (bind _asbp_patrol_locations (Utilities|Casting|CastToBP_PatrolLocations (Utilities|Array|Get(acopy) (Variables|Default|GetSearchRoute) (Variables|Default|GetPoint%20In%20Patrol)))
        (:then
          (LocalVariables|SetSetWaitTime (Variables|/Game/_SpiritTown/_AI/AIBase/BP_PatrolLocations.BP_PatrolLocations_C|GetWaittime _asbp_patrol_locations)))
        (:CastFailed
          (LocalVariables|SetSetWaitTime 0.5)))
      (return (LocalVariables|GetLastLocation) (LocalVariables|GetSetWaitTime) _asbp_patrol_locations))))