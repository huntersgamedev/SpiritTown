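; BP_PatrolLocations is an editor-configurable marker for AI locations, typed as either a regular patrol point or a search location.
; Its construction script switches on NodeType to set the PatrolLabel text component's color and text, so each type is visually distinct when placed.
; The event graph has no active logic, so the Blueprint itself runs no patrol or search behavior.
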(event EventBeginPlay)

(event Collision|EventActorBeginOverlap
  (params (OtherActor :type Actor%20Object%20Reference)))

(event EventTick
  (params (DeltaSeconds :type Float%20%28single-precision%29)))

(fn ConstructionScript
  (bind _patrollabel (Variables|Default|GetPatrolLabel))
  (bind _patrollabel_2 (Variables|Default|GetPatrolLabel))
  (switch Utilities|FlowControl|Switch|SwitchonNodeType (Variables|Default|GetNodeType)
    (:NewEnumerator0
      (Rendering|Components|TextRender|SetTextRenderColor _patrollabel_2 (Variables|Default|GetTextColor))
      (Rendering|Components|TextRender|SetText _patrollabel_2 (Variables|Default|GetPatrol%20Label)))
    (:NewEnumerator1
      (Rendering|Components|TextRender|SetTextRenderColor _patrollabel (Variables|Default|GetSearchColor))
      (Rendering|Components|TextRender|SetText _patrollabel (Variables|Default|GetSearchNode)))))