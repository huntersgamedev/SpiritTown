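; Stand-in actor that fades an object to translucent and back, copying mesh, materials and collision from a source static mesh component on construction.
; Opacity swaps in mapped or fallback translucent materials, then runs a timeline on the Opacity parameter at TraceToObjects rates.
; After fading back, or immediately if the out rate is non-positive, it restores the foliage instance transform or spawns a replacement StaticMeshActor, then destroys itself.
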(event Custom|Opacity
  (params (On :type Boolean))
  (bind _timeline_translucent (Variables|Default|GetTimeline_translucent))
  (bind _tracetoobjects (Variables|Default|GetTraceToObjects))
  (bind _smandindex (Variables|Default|GetSMandIndex))
  (bind _staticmesh (Variables|Default|GetStaticMesh))
  (bind _returnvalue (Collision|GetCollisionProfileName _staticmesh))
  (if On
    (for (_array_element _array_index) (Variables|Default|GetMaterials)
      (Rendering|Material|SetMaterial (Variables|Default|GetStaticMesh) _array_index (select (.ReturnValue (Utilities|Map|Find (Variables|Default|GetTableMaterial) _array_element)) (.Value (Utilities|Map|Find (Variables|Default|GetTableMaterial) _array_element)) "/Game/TUC/Materials/M_SimpleTransclucent.M_SimpleTransclucent")))
    (Variables|Default|SetComplite true)
    ;[1 1 1] OpacityTime
    (Components|Timeline|SetPlayRate _timeline_translucent (Variables|/Game/TUC/Blueprints/BP_TraceToObjects.BP_TraceToObjects_C|GetPlayRateIn _tracetoobjects))
    (bind (_direction _newtrack_0) (Timeline|Timeline_translucent Play)
      (:Update
        (Rendering|Material|SetScalarParameterValueonMaterials (Variables|Default|GetStaticMesh) "Opacity" (Math|Float|Lerp 1.0 0.15 _newtrack_0)))
      (:Finished
        (if (Utilities|Enum|Equal(Enum) _direction "Backward")
          (if (Variables|Default|GetFolliage) :!label _label
            ;[1 1 1] Folliage
            (Components|InstancedStaticMesh|UpdateInstanceTransform (.ism _smandindex) (.index _smandindex) (Transformation|GetActorTransform) false true true)
            (Actor|DestroyActor)
            (else
              ;[1 1 1] Only for UE4 v 4.21+
              (bind _returnvalue_2 (Game|SpawnActorfromClass "/Script/Engine.StaticMeshActor" (Transformation|GetActorTransform) "AlwaysSpawn" 0 0))
              (Transformation|SetMobility (Variables|/Script/Engine.StaticMeshActor|GetStaticMeshComponent _returnvalue_2) "Movable")
              (Collision|SetCollisionProfileName (Variables|/Script/Engine.StaticMeshActor|GetStaticMeshComponent _returnvalue_2) _returnvalue :!class /Script/Engine.PrimitiveComponent)
              (if (Utilities|Enum|Equal(Enum) (Utilities|String|ToString(Name) _returnvalue) "Custom")
                (CallFunction|SetCollision (Variables|Default|GetStaticMesh) (Variables|/Script/Engine.StaticMeshActor|GetStaticMeshComponent _returnvalue_2)))
              (Components|StaticMesh|SetStaticMesh (Variables|/Script/Engine.StaticMeshActor|GetStaticMeshComponent _returnvalue_2) (Variables|/Script/Engine.StaticMeshComponent|GetStaticMesh (Variables|Default|GetStaticMesh)))
              (for (_array_element_2 _array_index_2) (Variables|Default|GetMaterials)
                (Rendering|Material|SetMaterial (Variables|/Script/Engine.StaticMeshActor|GetStaticMeshComponent _returnvalue_2) _array_index_2 _array_element_2))
              (Actor|DestroyActor))))))
    (else
      (Variables|Default|SetComplite false)
      (if (<= (Variables|/Game/TUC/Blueprints/BP_TraceToObjects.BP_TraceToObjects_C|GetPlayRateOut (Variables|Default|GetTraceToObjects)) 0.0)
        (goto _label)
        (else
          (Components|Timeline|SetPlayRate _timeline_translucent (Variables|/Game/TUC/Blueprints/BP_TraceToObjects.BP_TraceToObjects_C|GetPlayRateOut _tracetoobjects))
          (Timeline|Timeline_translucent Reverse))))))

(event Custom|ReturnFolliage
  (bind _smandindex (Variables|Default|GetSMandIndex))
  ;[1 1 1] Folliage
  (Components|InstancedStaticMesh|UpdateInstanceTransform (.ism _smandindex) (.index _smandindex) (Transformation|GetActorTransform) false true true)
  (Actor|DestroyActor))

(fn ConstructionScript
  (bind _staticmesh (Variables|Default|GetStaticMesh))
  (bind _asstatic_mesh_component (Utilities|Casting|CastToStaticMeshComponent (Variables|Default|GetSM)))
  (Components|StaticMesh|SetStaticMesh _staticmesh (Variables|/Script/Engine.StaticMeshComponent|GetStaticMesh _asstatic_mesh_component))
  (Collision|SetCollisionProfileName _staticmesh (Collision|GetCollisionProfileName _asstatic_mesh_component) :!class /Script/Engine.PrimitiveComponent)
  (if (Utilities|Enum|Equal(Enum) (Utilities|String|ToString(Name) (Collision|GetCollisionProfileName _asstatic_mesh_component)) "Custom")
    (CallFunction|SetCollision _asstatic_mesh_component _staticmesh))
  (for (_array_element _array_index) (Variables|Default|GetMaterials)
    (Rendering|Material|SetMaterial (Variables|Default|GetStaticMesh) _array_index _array_element)))

(fn SetCollision
  (params (Old :type Static%20Mesh%20Component%20Object%20Reference) (New :type Static%20Mesh%20Component%20Object%20Reference))
  (Collision|SetCollisionResponsetoChannel New "ECC_WorldStatic" (Collision|GetCollisionResponsetoChannel Old "ECC_WorldStatic"))
  (Collision|SetCollisionResponsetoChannel New "ECC_WorldDynamic" (Collision|GetCollisionResponsetoChannel Old "ECC_WorldDynamic"))
  (Collision|SetCollisionResponsetoChannel New "ECC_Pawn" (Collision|GetCollisionResponsetoChannel Old "ECC_Pawn"))
  (Collision|SetCollisionResponsetoChannel New "ECC_Visibility" (Collision|GetCollisionResponsetoChannel Old "ECC_Visibility"))
  (Collision|SetCollisionResponsetoChannel New "ECC_Camera" (Collision|GetCollisionResponsetoChannel Old "ECC_Camera"))
  (Collision|SetCollisionResponsetoChannel New "ECC_PhysicsBody" (Collision|GetCollisionResponsetoChannel Old "ECC_PhysicsBody"))
  (Collision|SetCollisionResponsetoChannel New "ECC_Vehicle" (Collision|GetCollisionResponsetoChannel Old "ECC_Vehicle"))
  (Collision|SetCollisionResponsetoChannel New "ECC_Destructible" (Collision|GetCollisionResponsetoChannel Old "ECC_Destructible"))
  (return))