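; Helper actor that fades a group of static mesh actors sharing a tag to translucent, then restores them.
; Construction gathers actors with the second tag of SM's owner and saves their materials.
; Opacity on swaps in table-mapped materials or a simple translucent fallback, then a timeline lowers Opacity at TraceToObject's rate.
; Opacity off restores materials instantly, unregisters meshes from TraceToObject and destroys itself.
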(event Custom|Opacity
  (params (On :type Boolean))
  (bind _tracetoobject (Variables|Default|GetTraceToObject))
  (bind _smopacity (Variables|/Game/TUC/Blueprints/BP_TraceToObjects.BP_TraceToObjects_C|GetSMOpacity _tracetoobject))
  (if On
    ;[1 1 1] SetNewMaterials
    (for (_array_element _array_index) (Variables|Default|GetSMM)
      (for (_array_element_2 _array_index_2) (.materials _array_element)
        (bind _asstatic_mesh_component (Utilities|Casting|CastToStaticMeshComponent (Utilities|Array|Get(acopy) (Variables|Default|GetSMArray) _array_index)))
        (Rendering|Material|SetMaterial _asstatic_mesh_component _array_index_2 (select (.ReturnValue (Utilities|Map|Find (Variables|Default|GetTableMaterial) _array_element_2)) (.Value (Utilities|Map|Find (Variables|Default|GetTableMaterial) _array_element_2)) "/Game/TUC/Materials/M_SimpleTransclucent.M_SimpleTransclucent"))))
    ;[1 1 1] OpacityTime
    (Components|Timeline|SetPlayRate (Variables|Default|GetTimeline_translucent) (Variables|/Game/TUC/Blueprints/BP_TraceToObjects.BP_TraceToObjects_C|GetPlayRateIn (Variables|Default|GetTraceToObject)))
    (bind _newtrack_0 (Timeline|Timeline_translucent Play)
      (:Update
        (for _array_element_3 (Variables|Default|GetSMArray)
          (bind _asstatic_mesh_component_2 (Utilities|Casting|CastToStaticMeshComponent _array_element_3))
          (Rendering|Material|SetScalarParameterValueonMaterials _asstatic_mesh_component_2 "Opacity" (Math|Float|Lerp 1.0 0.15 _newtrack_0)))))
    (else
      ;[1 1 1] ReturnMaterials
      (for (_array_element_4 _array_index_3) (Variables|Default|GetSMM)
        (for (_array_element_5 _array_index_4) (.materials _array_element_4)
          (bind _asstatic_mesh_component_3 (Utilities|Casting|CastToStaticMeshComponent (Utilities|Array|Get(acopy) (Variables|Default|GetSMArray) _array_index_3)))
          (Rendering|Material|SetMaterial _asstatic_mesh_component_3 _array_index_4 _array_element_5)))
      (bind _outactors (Actor|GetAllActorswithTag (Utilities|Array|Get(acopy) (Variables|/Script/Engine.Actor|GetTags (Components|GetOwner (Utilities|Array|Get(acopy) (Variables|Default|GetSMArray)))) 1)))
      (for _array_element_6 _outactors
        (bind _asstatic_mesh_actor (Utilities|Casting|CastToStaticMeshActor _array_element_6))
        (Utilities|Array|RemoveIndex (Variables|/Game/TUC/Blueprints/BP_TraceToObjects.BP_TraceToObjects_C|GetSMM _tracetoobject) (Utilities|Array|FindItem _smopacity (Variables|/Script/Engine.StaticMeshActor|GetStaticMeshComponent _asstatic_mesh_actor)))
        (Utilities|Array|RemoveItem _smopacity (Variables|/Script/Engine.StaticMeshActor|GetStaticMeshComponent _asstatic_mesh_actor)))
      (Actor|DestroyActor))))

(fn ConstructionScript
  ;[1 1 1] SaveOldMaterials
  (bind _outactors (Actor|GetAllActorswithTag (Utilities|Array|Get(acopy) (Variables|/Script/Engine.Actor|GetTags (Components|GetOwner (Variables|Default|GetSM))) 1)))
  (for _array_element _outactors
    (bind _asstatic_mesh_actor (Utilities|Casting|CastToStaticMeshActor _array_element))
    (Utilities|Array|Add (Variables|Default|GetSMArray) (Variables|/Script/Engine.StaticMeshActor|GetStaticMeshComponent _asstatic_mesh_actor))
    (Utilities|Array|Add (Variables|Default|GetSMM) (Utilities|Struct|MakeSMMaterials (Rendering|Material|GetMaterials (Variables|/Script/Engine.StaticMeshActor|GetStaticMeshComponent _asstatic_mesh_actor))))))

(fn SetCollision
  (params (Old :type Static%20Mesh%20Component%20Object%20Reference) (New :type Static%20Mesh%20Component%20Object%20Reference))
  (Collision|SetCollisionResponsetoChannel New "ECC_WorldStatic" (Collision|GetCollisionResponsetoChannel Old "ECC_WorldStatic"))
  (Collision|SetCollisionResponsetoChannel New "ECC_WorldDynamic" (Collision|GetCollisionResponsetoChannel Old "ECC_WorldDynamic"))
  (Collision|SetCollisionResponsetoChannel New "ECC_Pawn" (Collision|GetCollisionResponsetoChannel Old "ECC_Pawn"))
  (Collision|SetCollisionResponsetoChannel New "ECC_Visibility" (Collision|GetCollisionResponsetoChannel Old "ECC_Visibility"))
  (Collision|SetCollisionResponsetoChannel New "ECC_Camera" (Collision|GetCollisionResponsetoChannel Old "ECC_Camera"))
  (Collision|SetCollisionResponsetoChannel New "ECC_PhysicsBody" (Collision|GetCollisionResponsetoChannel Old "ECC_PhysicsBody"))
  (Collision|SetCollisionResponsetoChannel New "ECC_Vehicle" (Collision|GetCollisionResponsetoChannel Old "ECC_Vehicle"))
  (Collision|SetCollisionResponsetoChannel New "ECC_Destructible" (Collision|GetCollisionResponsetoChannel Old "ECC_Destructible"))
  (return))