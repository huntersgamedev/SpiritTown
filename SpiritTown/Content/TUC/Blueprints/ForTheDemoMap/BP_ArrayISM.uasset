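; BP_ArrayISM is a demo-map actor that builds a cubic grid of small, evenly spaced static meshes in its construction script.
; Three nested loops place the meshes, and the Instance flag selects how each one is created.
; When set, it adds world-space instances to one InstancedStaticMesh, offset by actor location but ignoring actor rotation.
; Otherwise, it adds a separate StaticMeshComponent per cell in relative space.
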(fn ConstructionScript
  (for _index (range 0 4)
    (for _index_2 (range 0 4)
      (for _index_3 (range 0 4)
        (if (Variables|Default|GetInstance?)
          (Class|InstancedStaticMeshComponent|AddInstanceWorldSpace (Variables|Default|GetInstancedStaticMesh) (Math|Transform|MakeTransform (+ (Math|Vector|MakeVector (* _index 5e+01) (* _index_2 5e+01) (* _index_3 5e+01)) (Transformation|GetActorLocation)) "0, 0, 0" "0.100000,0.100000,0.100000"))
          (else
            (AddComponent|AddStaticMeshComponent false (Math|Transform|MakeTransform (Math|Vector|MakeVector (* _index 5e+01) (* _index_2 5e+01) (* _index_3 5e+01)) "0, 0, 0" "0.100000,0.100000,0.100000"))))))))