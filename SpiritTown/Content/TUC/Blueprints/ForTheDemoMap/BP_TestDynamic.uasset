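; BP_TestDynamic is a test Blueprint, filed under the demo map, whose Cube component shuttles endlessly back and forth along its relative X axis.
; BeginPlay starts two looping wire chains that hand off to each other at the travel limits.
; Each step is a one-unit swept move followed by a zero-length Delay that yields a frame, so speed depends on frame rate and no Tick event is used.
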(event EventBeginPlay
  (Transformation|AddRelativeLocation (Variables|Default|GetCube) "1.000000, 0, 0" true false :!label _label)
  (Utilities|FlowControl|Delay 0.0)
  (if (>= (.x (Variables|/Script/Engine.SceneComponent|GetRelativeLocation (Variables|Default|GetCube))) 3.5e+02)
    (Transformation|AddRelativeLocation (Variables|Default|GetCube) "-1.000000, 0, 0" true false :!label _label_2)
    (Utilities|FlowControl|Delay 0.0)
    (if (<= (.x (Variables|/Script/Engine.SceneComponent|GetRelativeLocation (Variables|Default|GetCube))) 0.0)
      (goto _label)
      (else
        (goto _label_2)))
    (else
      (goto _label))))

(fn ConstructionScript)